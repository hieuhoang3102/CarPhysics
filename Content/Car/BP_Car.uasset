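; BP_Car is an early car actor whose only working behavior is a debug R key that resets its rotation to zero.
; An unfinished Suspension function sketches raycast springs: trace down from a wheel component, then push the Box along the trace at that point, scaled by compression and Strength.
; That logic is disconnected from the function entry, and nothing in the file calls Suspension, so no suspension force is applied.
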(event EventBeginPlay)

(event Collision|EventActorBeginOverlap
  (params (OtherActor :type Actor%20Object%20Reference)))

(event Input|KeyboardEvents|DebugKeyR
  (params (Key :type Key%20Structure :default "None") (ActionValue :type Input%20Action%20Value%20Structure))
  (:Pressed
    (Transformation|SetActorRotation "0, 0, 0")))

(fn ConstructionScript)

(fn Suspension
  (params (Wheel%20Scene :type Scene%20Component%20Object%20Reference)))